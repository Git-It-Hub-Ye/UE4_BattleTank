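; Player-controlled tank vehicle that lets input aim its turret and barrel.
; On BeginPlay it initialises its aiming component with the Barrel, the Turret and itself as owner.
; The AimRotation and AimElevation input axes pass their values straight to the turret's rotation and the barrel's elevation functions.
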(event `self.ReceiveBeginPlay`
  (`AimingComponent.Initialise` (`self.AimingComp`) (`self.Barrel`) (`self.Turret`) self))

(event `InputAxis|AimRotation`
  (params (AxisValue :type "Float (single-precision)"))
  (`Turret.RotateTurret` (`self.Turret`) AxisValue))

(event `InputAxis|AimElevation`
  (params (AxisValue :type "Float (single-precision)"))
  (`Barrel.ElevateBarrel` (`self.Barrel`) AxisValue))

(fn `UserConstructionScript`)