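; BP_PlayerTank is the player-controlled tank Blueprint, wiring input to its aiming and movement parts.
; On BeginPlay it initialises the aiming component with the barrel, turret and itself, and the movement component with both tracks.
; Aim axes directly elevate the barrel and rotate the turret, while drive axes pass forward and turn intents to the movement component.
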(event `self.ReceiveBeginPlay`
  (`AimingComponent.Initialise` (`self.AimingComp`) (`self.Barrel`) (`self.Turret`) self)
  (`TankMovement.Initialise` (`self.TankMovement`) (`self.LeftTrack`) (`self.RightTrack`)))

(event `InputAxis|AimElevation`
  (params (AxisValue :type "Float (single-precision)"))
  (`Barrel.ElevateBarrel` (`self.Barrel`) AxisValue))

(event `InputAxis|AimRotation`
  (params (AxisValue :type "Float (single-precision)"))
  (`Turret.RotateTurret` (`self.Turret`) AxisValue))

(event `InputAxis|MoveForward`
  (params (AxisValue :type "Float (single-precision)"))
  (`TankMovement.IntendMoveForward` (`self.TankMovement`) AxisValue))

(event `InputAxis|TurnRight`
  (params (AxisValue :type "Float (single-precision)"))
  (`TankMovement.IntendTurnRight` (`self.TankMovement`) AxisValue))

(fn `UserConstructionScript`)