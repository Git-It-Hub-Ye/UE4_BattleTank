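; Blueprint for an AI tank that wires up its aiming and movement components and silences itself when destroyed.
; On BeginPlay it initialises the aiming component with barrel and turret and the movement component with both tracks.
; The tank destroyed event calls a helper that, when true, stops engine, turret and barrel audio and halts aiming actions.
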(event `self.ReceiveBeginPlay`
  (`AimingComponent.Initialise` (`self.AimingComp`) (`self.Barrel`) (`self.Turret`) self)
  (`TankMovement.Initialise` (`self.MovementComp`) (`self.LeftTrack`) (`self.RightTrack`)))

(event `self.OnTankDestroyed`
  (params (bDestroyed :type Boolean))
  (`self.StopAudioOnTank` bDestroyed))

(fn `StopAudioOnTank`
  (params (Condition :type Boolean))
  (if Condition
    (`TankMovement.StopEngineSound` (`self.MovementComp`))
    (`Turret.StopTurretAudio` (`self.Turret`))
    (`Barrel.StopBarrelAudio` (`self.Barrel`))
    (`AimingComponent.StopActions` (`self.AimingComp`))))

(fn `UserConstructionScript`)